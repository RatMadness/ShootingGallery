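; BP_Player is a player Blueprint that snaps the player pawn between three fixed positions side by side along the Y axis.
; The Q, W and E keys each set the actor transform directly, without sweeping, to the left, middle or right spot.
; Each key gets its target through an interface message on player pawn 0, which this Blueprint implements in SetPlayerRef by returning itself.
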(event `Key|Q`
  (params (Key :type "Key Structure"))
  (:`Pressed`
    (bind _player (message `/Game/Interfaces/INT_Player.SetPlayerRef` (`GameplayStatics.GetPlayerPawn` 0)))
    (`self.K2_SetActorTransform` _player (`KismetMathLibrary.MakeTransform` (-520.0 -250.0 112.0)) false false)))

(event `Key|W`
  (params (Key :type "Key Structure"))
  (:`Pressed`
    (bind _player (message `/Game/Interfaces/INT_Player.SetPlayerRef` (`GameplayStatics.GetPlayerPawn` 0)))
    (`self.K2_SetActorTransform` _player (`KismetMathLibrary.MakeTransform` (-520.0 10.0 112.0)) false false)))

(event `Key|E`
  (params (Key :type "Key Structure"))
  (:`Pressed`
    (bind _player (message `/Game/Interfaces/INT_Player.SetPlayerRef` (`GameplayStatics.GetPlayerPawn` 0)))
    (`self.K2_SetActorTransform` _player (`KismetMathLibrary.MakeTransform` (-520.0 250.0 112.0)) false false)))

(fn `SetPlayerRef`
  (returns (Player :type "/Game/Blueprints/BP_Player Object Reference"))
  (return self))

(fn `UserConstructionScript`)